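; BP_PlayerController is a player controller that turns player input into commands for the pawn it controls.
; Axis inputs for movement and looking, plus Jump, Run and ChangeWeapon actions, are forwarded to the controlled pawn as interface messages, with press and release mapped to start and stop for Jump and Run.
; The controller holds no gameplay logic, so each pawn decides how to respond without the controller casting to a specific class.
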(event Input|ActionEvents|InputActionJump
  (params (Key :type Key%20Structure :default "None"))
  (bind _returnvalue (Pawn|GetControlledPawn))
  (:Pressed
    (Class|BPInterface|StartJump(Message) _returnvalue))
  (:Released
    (Class|BPInterface|EndJump(Message) _returnvalue)))

(event Input|ActionEvents|InputActionChangeWeapon
  (params (Key :type Key%20Structure :default "None"))
  (:Pressed
    (Class|BPInterface|ChangeWeapon(Message) (Pawn|GetControlledPawn))))

(event Input|ActionEvents|InputActionRun
  (params (Key :type Key%20Structure :default "None"))
  (bind _returnvalue (Pawn|GetControlledPawn))
  (:Pressed
    (Class|BPInterface|StartRun(Message) _returnvalue))
  (:Released
    (Class|BPInterface|StopRun(Message) _returnvalue)))

(event Input|AxisEvents|InputAxisMoveForward
  (params (AxisValue :type Float%20%28single-precision%29))
  (Class|BPInterface|MoveForward(Message) (Pawn|GetControlledPawn) AxisValue))

(event Input|AxisEvents|InputAxisMoveRight
  (params (AxisValue :type Float%20%28single-precision%29))
  (Class|BPInterface|MoveRight(Message) (Pawn|GetControlledPawn) AxisValue))

(event Input|AxisEvents|InputAxisLookUp
  (params (AxisValue :type Float%20%28single-precision%29))
  (Class|BPInterface|LookUp(Message) (Pawn|GetControlledPawn) AxisValue))

(event Input|AxisEvents|InputAxisTurn
  (params (AxisValue :type Float%20%28single-precision%29))
  (Class|BPInterface|Turn(Message) (Pawn|GetControlledPawn) AxisValue))

(fn ConstructionScript)