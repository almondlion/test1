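; CombatArea is a Blueprint box trigger that switches the player into and out of combat.
; Entering the box sets IsCombat on BP_Player and calls StartCombat after a half-second delay.
; Leaving clears the flag and calls EndCombat after the same delay.
; Two DoOnce gates reset each other on opposite overlap events, so each transition fires once until the player crosses back.
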(event OnComponentBeginOverlap(Box)
  (params (OverlappedComponent :type Primitive%20Component%20Object%20Reference) (OtherActor :type Actor%20Object%20Reference) (OtherComp :type Primitive%20Component%20Object%20Reference) (OtherBodyIndex :type Integer) (bFromSweep :type Boolean) (SweepResult :type Hit%20Result%20Structure%20%28by%20ref%29))
  (bind _asbp_player (Utilities|Casting|CastToBP_Player OtherActor))
  (Utilities|FlowControl|Sequence
    (:then_0
      (Utilities|FlowControl|DoOnce false
        (:Completed
          (Variables|/Game/BluePrints/BP_Base.BP_Base_C|SetIsCombat _asbp_player true)
          (Utilities|FlowControl|Delay 0.5)
          (Default|StartCombat _asbp_player))))
    (:then_1
      (Utilities|FlowControl|DoOnce false) ; enters at Reset
    )))

(event OnComponentEndOverlap(Box)
  (params (OverlappedComponent :type Primitive%20Component%20Object%20Reference) (OtherActor :type Actor%20Object%20Reference) (OtherComp :type Primitive%20Component%20Object%20Reference) (OtherBodyIndex :type Integer))
  (bind _asbp_player (Utilities|Casting|CastToBP_Player OtherActor))
  (Utilities|FlowControl|Sequence
    (:then_0
      (Utilities|FlowControl|DoOnce false
        (:Completed
          (Variables|/Game/BluePrints/BP_Base.BP_Base_C|SetIsCombat _asbp_player false)
          (Utilities|FlowControl|Delay 0.5)
          (Default|EndCombat _asbp_player))))
    (:then_1
      (Utilities|FlowControl|DoOnce false) ; enters at Reset
    )))

(fn ConstructionScript)