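; Base character with camera-relative movement, katana draw and sheathe, section-cycling attacks, and a context-dependent run/dodge action.
; BeginPlay attaches a spawned katana and starts a looping timer measuring movement-input angle against actor facing.
; In combat with katana drawn, that angle picks a directional root-motion dodge; otherwise, outside combat, a reversible timeline ramps walk speed, camera lag and particle spawn rate.
; CanMotion gates weapon swaps, allowed only when nearly stationary, and dodges.
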(event Custom|SetDirection
  (bind _returnvalue (Pawn|GetControlRotation :!class /Script/Engine.Pawn))
  (bind _yaw (Math|Rotator|BreakRotator _returnvalue))
  (bind _returnvalue_2 (Math|Rotator|MakeRotator 0.0 0.0 _yaw))
  (Variables|Default|SetZ%20%28Yaw%29 (Math|Float|SelectFloat 0.0 (.Yaw (Math|Rotator|BreakRotator (Math|Rotator|Delta(Rotator) (Math|Conversions|RotationFromXVector (+ (* (Variables|Default|GetMoveF) (Math|Vector|GetForwardVector _returnvalue_2)) (* (Variables|Default|GetMoveR) (Math|Vector|GetRightVector _returnvalue_2)))) (Transformation|GetActorRotation)))) (== (+ (Math|Float|Absolute(Float) (Variables|Default|GetMoveF)) (Math|Float|Absolute(Float) (Variables|Default|GetMoveR))) 0.0))))

(event Custom|StartCombat
  (if (not (Variables|Default|GetIsKatana))
    ;[1 1 1] 拔刀
    (bind _returnvalue (Animation|PlayAnimMontage "/Game/GhostSamurai_Bundle/GhostSamurai/Katana/Common/Inplace/GhostSamurai_APose_Equip01_Inplace_Montage.GhostSamurai_APose_Equip01_Inplace_Montage" 1.2 "None"))
    (Variables|Default|SetIsKatana true)
    (Utilities|FlowControl|Delay _returnvalue)
    (Variables|Default|SetCanMotion true)))

(event Custom|EndCombat
  (if (Variables|Default|GetIsKatana)
    ;[1 1 1] 收刀
    (bind _returnvalue (Animation|PlayAnimMontage "/Game/GhostSamurai_Bundle/GhostSamurai/Katana/Common/Root/GhostSamurai_APose_Unarm_3_Root_Montage.GhostSamurai_APose_Unarm_3_Root_Montage" 1.2 "None"))
    (Variables|Default|SetIsKatana false)
    (Utilities|FlowControl|Delay _returnvalue)
    (Variables|Default|SetCanMotion true)))

(event EventAttack
  (Animation|PlayAnimMontage "/Game/GhostSamurai_Bundle/GhostSamurai/Katana/Apose/Attack/Root/GhostSamurai_APose_Attack01_1_ALL_Root_Montage.GhostSamurai_APose_Attack01_1_ALL_Root_Montage" 1.0 (Utilities|Array|Get(acopy) (Variables|Default|GetAttackSection) (Variables|Default|GetAttackIndex)))
  (bind _result (Math|Integer|IncrementInt (Variables|Default|GetAttackIndex))
    (:%20%20
      (Math|Integer|CompareInt _result 4
        (:>
          _)
        (:==
          _))
      (Variables|Default|SetAttackIndex 0))))

(event EventBeginPlay
  (Utilities|Time|SetTimerbyEvent (delegate Custom|SetDirection) 0.01 true)
  (bind _returnvalue (Game|SpawnActorfromClass "/Game/BluePrints/Weapon/BP_Katana.BP_Katana_C" (Math|Transform|MakeTransform "0, 0, 0" "0, 0, 0" "1.000000,1.000000,1.000000") "Undefined" 0 0))
  (bind _output_get (Variables|Default|SetKatana _returnvalue))
  (Transformation|AttachComponentToComponent _output_get (Variables|Character|GetMesh) "katana_Targer01" "SnapToTarget" "SnapToTarget" "SnapToTarget" true)
  (Collision|SetCollisionEnabled (Variables|/Game/BluePrints/Weapon/BP_Katana.BP_Katana_C|GetKatana _output_get) "NoCollision"))

(event EventChangeWeapon
  ;[1 1 1] 因为改了mesh导致移动时武器错位所以让移动时无法拔刀
  (if (< (Math|Vector|VectorLength (Transformation|GetVelocity)) 1e+01)
    ;[1 1 1] 让动画播放的时候不被打断
    (if (Variables|Default|GetCanMotion)
      (Variables|Default|SetCanMotion false)
      (if (Variables|Default|GetIsKatana)
        ;[1 1 1] 收刀
        (bind _returnvalue (Animation|PlayAnimMontage "/Game/GhostSamurai_Bundle/GhostSamurai/Katana/Common/Root/GhostSamurai_APose_Unarm_3_Root_Montage.GhostSamurai_APose_Unarm_3_Root_Montage" 1.2 "None"))
        (Variables|Default|SetIsKatana false)
        (Utilities|FlowControl|Delay _returnvalue)
        (Variables|Default|SetCanMotion true)
        (else
          ;[1 1 1] 拔刀
          (bind _returnvalue_2 (Animation|PlayAnimMontage "/Game/GhostSamurai_Bundle/GhostSamurai/Katana/Common/Inplace/GhostSamurai_APose_Equip01_Inplace_Montage.GhostSamurai_APose_Equip01_Inplace_Montage" 1.2 "None"))
          (Variables|Default|SetIsKatana true)
          (Utilities|FlowControl|Delay _returnvalue_2)
          (Variables|Default|SetCanMotion true))))))

(event EventStartRun
  ;[1 1 1] 战斗状态下翻滚，非战斗状态下快跑
  (if (Variables|Default|GetIsCombat)
    ;[1 1 1] 拔刀状态下才能翻滚
    (if (Variables|Default|GetIsKatana)
      ;[1 1 1] 防止连续翻滚
      (if (Variables|Default|GetCanMotion)
        (Variables|Default|SetCanMotion false)
        (if (Math|Float|InRange(Float) (Variables|Default|GetZ%20%28Yaw%29) -45.0 45.0)
          (Animation|PlayAnimMontage "/Game/GhostSamurai_Bundle/GhostSamurai/Katana/Apose/Dodge/Root/GhostSamurai_APose_Dodge_F_Root_Montage.GhostSamurai_APose_Dodge_F_Root_Montage" 1.2 "None")
          (elif (Math|Float|InRange(Float) (Variables|Default|GetZ%20%28Yaw%29) -135.0 -45.0)
            (Animation|PlayAnimMontage "/Game/GhostSamurai_Bundle/GhostSamurai/Katana/Apose/Dodge/Root/GhostSamurai_APose_Dodge_L_Root_Montage.GhostSamurai_APose_Dodge_L_Root_Montage" 1.2 "None")
            (elif (Math|Float|InRange(Float) (Variables|Default|GetZ%20%28Yaw%29) 45.0 135.0)
              (Animation|PlayAnimMontage "/Game/GhostSamurai_Bundle/GhostSamurai/Katana/Apose/Dodge/Root/GhostSamurai_APose_Dodge_R_Root_Montage.GhostSamurai_APose_Dodge_R_Root_Montage" 1.2 "None")
              (else
                (Animation|PlayAnimMontage "/Game/GhostSamurai_Bundle/GhostSamurai/Katana/Apose/Dodge/Root/GhostSamurai_APose_Dodge_B_Root_Montage.GhostSamurai_APose_Dodge_B_Root_Montage" 1.2 "None")))))))
    (else
      (Variables|Default|SetRunning true)
      (bind (_direction _newtrack_0 _newtrack_1 _newtrack_2) (Timeline|Timeline_0 Play)
        (:Update
          ;[1 1 1] 移速、摄像头距离和特效都进行3秒的渐变效果
          (Variables|/Script/Engine.CharacterMovementComponent|SetMaxWalkSpeed (Variables|Character|GetCharacterMovement) _newtrack_0)
          (Variables|/Script/Engine.SpringArmComponent|SetCameraLagSpeed (Variables|Default|GetSpringArm) _newtrack_1)
          (Niagara|SetNiagaraVariable(Float) (Variables|Default|GetNE_RunningEmitter_System) "SpawnRate" _newtrack_2))))))

(event EventMoveForward
  (params (Value :type Float%20%28double-precision%29))
  (Pawn|Input|AddMovementInput (Math|Vector|GetForwardVector (Math|Rotator|MakeRotator 0.0 0.0 (.Yaw (Math|Rotator|BreakRotator (Pawn|GetControlRotation :!class /Script/Engine.Pawn))))) Value false)
  (Variables|Default|SetMoveF Value))

(event EventMoveRight
  (params (Value :type Float%20%28double-precision%29))
  (Pawn|Input|AddMovementInput (Math|Vector|GetRightVector (Math|Rotator|MakeRotator 0.0 0.0 (.Yaw (Math|Rotator|BreakRotator (Pawn|GetControlRotation :!class /Script/Engine.Pawn))))) Value false)
  (Variables|Default|SetMoveR Value))

(event EventTurn
  (params (Value :type Float%20%28double-precision%29))
  (Pawn|Input|AddControllerYawInput (Math|Float|SelectFloat (* Value 0.2) Value (Variables|Default|GetRunning))))

(event EventLookUp
  (params (Value :type Float%20%28double-precision%29))
  (Pawn|Input|AddControllerPitchInput (Math|Float|SelectFloat (* Value 0.2) Value (Variables|Default|GetRunning))))

(event EventStartJump
  (Character|Jump))

(event EventEndJump
  (Character|StopJumping))

(event EventStopRun
  ;[1 1 1] 战斗状态下翻滚，非战斗状态下快跑
  (if (not (Variables|Default|GetIsCombat))
    (Variables|Default|SetRunning false)
    (bind (_direction _newtrack_0 _newtrack_1 _newtrack_2) (Timeline|Timeline_0 Reverse)
      (:Update
        ;[1 1 1] 移速、摄像头距离和特效都进行3秒的渐变效果
        (Variables|/Script/Engine.CharacterMovementComponent|SetMaxWalkSpeed (Variables|Character|GetCharacterMovement) _newtrack_0)
        (Variables|/Script/Engine.SpringArmComponent|SetCameraLagSpeed (Variables|Default|GetSpringArm) _newtrack_1)
        (Niagara|SetNiagaraVariable(Float) (Variables|Default|GetNE_RunningEmitter_System) "SpawnRate" _newtrack_2)))))

(fn ConstructionScript)