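; Behavior tree service that detects the player for an AI pawn by a facing-angle check.
; Each tick it compares the pawn's forward vector with the direction to player 0, using a dot product and arccosine.
; Within a 45 degree half-angle, it writes the player and a true tracing flag to the blackboard.
; It tests neither distance nor line of sight and never clears either key.
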(event EventReceiveTickAI
  (params (OwnerController :type AI%20Controller%20Object%20Reference) (ControlledPawn :type Pawn%20Object%20Reference) (DeltaSeconds :type Float%20%28single-precision%29))
  (bind _returnvalue (Game|Player|GetPlayerPawn 0))
  (if (< (Class|KismetMathLibrary|DegAcos (Math|Vector|DotProduct (Math|Vector|Normalize (- (Transformation|GetActorLocation _returnvalue) (Transformation|GetActorLocation ControlledPawn))) (Transformation|GetActorForwardVector ControlledPawn))) 45.0)
    (Class|BTFunctionLibrary|SetBlackboardValueasObject (Variables|Default|GetPlayerKey) _returnvalue)
    (Class|BTFunctionLibrary|SetBlackboardValueasBool (Variables|Default|GetTracingKey) true)))